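; Anim notify state that lets a character rotate through movement physics during a root motion animation window.
; On begin it casts the mesh owner to Character and enables AllowPhysicsRotationDuringAnimRootMotion on its CharacterMovement.
; On end it sets the flag back to false rather than restoring the previous value.
; Both events return false when the owner is not a Character or has no valid movement component.
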(fn ReceivedNotifyBegin
  (params (MeshComp :type Skeletal%20Mesh%20Component%20Object%20Reference) (Animation :type Anim%20Sequence%20Base%20Object%20Reference) (TotalDuration :type Float%20%28single-precision%29) (EventReference :type Anim%20Notify%20Event%20Reference%20Structure%20%28by%20ref%29))
  (bind _ascharacter (Utilities|Casting|CastToCharacter (Components|GetOwner MeshComp))
    (:then
      (Utilities|IsValid (Variables|/Script/Engine.Character|GetCharacterMovement _ascharacter)
        (:Is%20Valid
          (Variables|/Script/Engine.CharacterMovementComponent|SetbAllowPhysicsRotationDuringAnimRootMotion (Variables|/Script/Engine.Character|GetCharacterMovement _ascharacter) true)
          (return true))
        (:Is%20Not%20Valid
          _)))
    (:CastFailed
      _))
  (return false))

(fn ReceivedNotifyEnd
  (params (MeshComp :type Skeletal%20Mesh%20Component%20Object%20Reference) (Animation :type Anim%20Sequence%20Base%20Object%20Reference) (EventReference :type Anim%20Notify%20Event%20Reference%20Structure%20%28by%20ref%29))
  (bind _ascharacter (Utilities|Casting|CastToCharacter (Components|GetOwner MeshComp))
    (:then
      (Utilities|IsValid (Variables|/Script/Engine.Character|GetCharacterMovement _ascharacter)
        (:Is%20Valid
          (Variables|/Script/Engine.CharacterMovementComponent|SetbAllowPhysicsRotationDuringAnimRootMotion (Variables|/Script/Engine.Character|GetCharacterMovement _ascharacter) false)
          (return true))
        (:Is%20Not%20Valid
          _)))
    (:CastFailed
      _))
  (return false))