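; BP_HoverTextActor is a floating NPC dialogue text actor that shows a bird character's joke lines.
; On BeginPlay it writes its current text to a TextRender, and every tick it smoothly rotates to face the player character.
; NextDialog picks a hard-coded line by dialogue number, ending on an empty one, while SetBlank and NextPosition let callers clear or move the text.
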(event EventBeginPlay
  (Rendering|Components|TextRender|SetText (Variables|Default|GetTextRender) (Variables|Default|GetCurrentTextReal)))

(event Collision|EventActorBeginOverlap
  (params (OtherActor :type Actor%20Object%20Reference)))

(event EventTick
  (params (DeltaSeconds :type Float%20%28single-precision%29))
  (Transformation|SetActorRotation (Math|Interpolation|RInterpTo (Transformation|GetActorRotation) (Math|Rotator|FindLookatRotation (Transformation|GetActorLocation) (Transformation|GetActorLocation (Game|GetPlayerCharacter 0))) (Utilities|Time|GetWorldDeltaSeconds) 2.0)))

(event EventNextDialog
  (params (DialogueNumber :type Integer))
  (Variables|Default|SetCurrentTextNum (+ (Variables|Default|GetCurrentTextNum) 1))
  (switch int DialogueNumber
    (:Default
      _)
    (:0
      (Variables|Default|SetCurrentTextReal "squack squak  
 
(with rizz)"))
    (:1
      (Variables|Default|SetCurrentTextReal "*starts breakdancing*"))
    (:2
      (Variables|Default|SetCurrentTextReal "You gotta help me, it's me Keanu Reeves 
and I'm trapped inside this bird 
 
*starts breakdancing*"))
    (:3
      (Variables|Default|SetCurrentTextReal "*heh* 
you know kid... you're alright... 
now... 
how about you say we make this banner fall? 
 
 
*starts breakdancing*"))
    (:4
      (Variables|Default|SetCurrentTextReal "")))
  (Rendering|Components|TextRender|SetText (Variables|Default|GetTextRender) (Variables|Default|GetCurrentTextReal)))

(event EventSetBlank
  (Rendering|Components|TextRender|SetText (Variables|Default|GetTextRender) (Variables|Default|GetBlankText)))

(event EventNextPosition
  (params (NewPos :type Vector :default "0, 0, 0"))
  (Transformation|SetActorLocation NewPos false false))

(fn ConstructionScript)