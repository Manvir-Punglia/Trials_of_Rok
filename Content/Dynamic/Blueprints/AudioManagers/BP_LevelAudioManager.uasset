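; BP_LevelAudioManager is a level music manager that plays a test theme on BeginPlay and switches between music phases.
; It creates one audio component, CurrentTrack, and reuses it for every sound through PlaySound.
; BeginPhase fades out the current track, waits the fade duration on a timer, then plays the supplied intro.
; When the intro finishes, an audio-finished binding starts the loop cue and unbinds itself.
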(event Custom|PlaySound
  (params (NewParam :type Sound%20Cue%20Object%20Reference))
  (bind _currenttrack (Variables|Default|GetCurrentTrack))
  ;[1 1 1] Plays a new Sound
  (Audio|Components|Audio|SetSound _currenttrack NewParam)
  (Audio|Components|Audio|Play _currenttrack 0.0))

(event Custom|BeginPhase
  (params (Intro :type Sound%20Cue%20Object%20Reference) (Loop :type Sound%20Cue%20Object%20Reference))
  (bind _fadeoutduration (Variables|Default|GetfadeOutDuration))
  ;[1 1 1] Call to start a new phase of music, requires intro + loop of phase                                   IDEA: called when boss first spots player in boss script, then called when boss enters phase 2
  (Development|PrintString "Beginning a new Phase")
  (Audio|Components|Audio|FadeOut (Variables|Default|GetCurrentTrack) _fadeoutduration 0.0 "Linear" :!class /Script/Engine.AudioComponent)
  (Utilities|Time|SetTimerbyEvent (delegate Custom|BeginPhase1TimerEvent) _fadeoutduration))

(event Custom|BeginPhase1TimerEvent
  ;[1 1 1] Call to start a new phase of music, requires intro + loop of phase                                   IDEA: called when boss first spots player in boss script, then called when boss enters phase 2
  (CallFunction|PlaySound (stale Custom|BeginPhase Intro))
  (EventDispatchers|BindEventtoOnAudioFinished (Variables|Default|GetCurrentTrack) (delegate Custom|OnAudioEventFinished_Event)))

(event Custom|OnAudioEventFinished_Event
  ;[1 1 1] Call to start a new phase of music, requires intro + loop of phase                                   IDEA: called when boss first spots player in boss script, then called when boss enters phase 2
  (CallFunction|PlaySound (stale Custom|BeginPhase Loop))
  (EventDispatchers|UnbindallEventsfromOnAudioFinished (Variables|Default|GetCurrentTrack))
  (Development|PrintString "playing loop"))

(event EventBeginPlay
  ;[1 1 1] creates audio component, sets internal reference to it, begins playing level theme.                                                  Begins first phase; placeholder
  (bind _returnvalue (AddComponent|AddAudioComponent false))
  (Variables|Default|SetCurrentTrack _returnvalue)
  (CallFunction|PlaySound "/Game/Dynamic/Music/Begin_Your_Trials_TEST_Cue.Begin_Your_Trials_TEST_Cue"))

(event Collision|EventActorBeginOverlap
  (params (OtherActor :type Actor%20Object%20Reference)))

(event EventTick
  (params (DeltaSeconds :type Float%20%28single-precision%29)))

(fn ConstructionScript)