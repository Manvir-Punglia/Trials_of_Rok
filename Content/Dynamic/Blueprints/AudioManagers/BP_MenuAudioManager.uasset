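; Menu audio manager that starts a layered music track and plays a sound for menu button hovers.
; BeginPlay adds an audio component and fires six SetGain trigger parameters on it to bring in the layers.
; PlayHoverCue only plays a 2D hover sound, ignoring its cue number.
; StopHoverCue and FadeOutEverything are empty, and the per-button layer switching logic is disconnected, so it never runs.
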(event Custom|PlayHoverCue
  (params (cueNum :type Integer))
  ;[1 1 1] plays specific layers based on int being fed into event, each menu button corresponds to a different int
  (Audio|PlaySound2D "/Game/Dynamic/SoundEffects/Menu/hover_Cue.hover_Cue" 1.0 1.0 0.0 0 0))

(event Custom|StopHoverCue
  (params (Cue%20Num :type Integer))
  ;[1 1 1] stops playing layers based on int fed into event, plays when no longer hovering a button
)

(event Custom|FadeOutEverything
  ;[1 1 1] fades every layer out
)

(event EventBeginPlay
  ;[1 1 1] creates audio component of track with multiple layers and plays initial layers
  (bind _returnvalue (AddComponent|AddAudioComponent false))
  (bind _output_get (Variables|Default|SetMenuComp _returnvalue))
  (Class|AudioParameterControllerInterface|SetTriggerParameter _output_get "SetGain1")
  (Class|AudioParameterControllerInterface|SetTriggerParameter _output_get "SetGain2")
  (Class|AudioParameterControllerInterface|SetTriggerParameter _output_get "SetGain3")
  (Class|AudioParameterControllerInterface|SetTriggerParameter _output_get "SetGain4")
  (Class|AudioParameterControllerInterface|SetTriggerParameter _output_get "SetGain5")
  (Class|AudioParameterControllerInterface|SetTriggerParameter _output_get "SetGain6"))

(fn ConstructionScript)