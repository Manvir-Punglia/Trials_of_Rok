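; One-shot tutorial trigger actor that moves the tutorial bird NPC and changes its dialogue when the player reaches it.
; On BeginPlay it caches the BP_TutorialEventManager found in the level.
; An overlap by BP_ThirdPersonCharacter sends its bird position and dialogue number to the manager through the tutorial events interface's CollisionEvent, then destroys the trigger.
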(event Custom|Collision
  ;[1 1 1] When called, executes the CollisionEvent function in the tutorial events interface on the tutorial manager and sends the NPC's new position and dialogue value  then destroys itself
  (Default|CollisionEvent (Variables|Default|GetTutorialManagerRef) (Variables|Default|GetBirdPos) (Variables|Default|GetDialogueNum))
  (Actor|DestroyActor))

(event Collision|EventActorBeginOverlap
  (params (OtherActor :type Actor%20Object%20Reference))
  ;[1 1 1] when something collides with this object that has the ThirdPersonCharacter's class, execute collision event
  (if (== (Utilities|GetClass OtherActor) "/Game/Dynamic/Blueprints/Character_BP/BP_ThirdPersonCharacter.BP_ThirdPersonCharacter_C")
    (CallFunction|Collision)))

(event EventBeginPlay
  ;[1 1 1] Stores reference to tutorial event manager on begin
  (bind _returnvalue (Actor|GetActorOfClass "/Game/Dynamic/Blueprints/TutorialObjects/BP_TutorialEventManager.BP_TutorialEventManager_C"))
  (Variables|Default|SetTutorialManagerRef _returnvalue))

(fn ConstructionScript)