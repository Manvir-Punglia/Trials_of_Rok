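; Field system actor in the tutorial objects that sets the Chaos physics dynamic state using a box-shaped culling field.
; The construction script adds a command that masks a uniform Dynamic state value with the Box component's falloff, culling inside the box.
; On actor overlap, it resets the field system and adds the same command again from the box's current transform.
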(event EventBeginPlay)

(event Collision|EventActorBeginOverlap
  (params (OtherActor :type Actor%20Object%20Reference))
  (Class|FieldSystemComponent|ResetFieldSystem (Variables|Field|GetFieldSystemComponent))
  (Class|FieldSystemComponent|AddFieldCommand (Variables|Field|GetFieldSystemComponent) true "Field_DynamicState" 0 (Field|SetCullingField (Variables|Default|GetCullingField) (Field|SetBoxFalloff (Variables|Default|GetBoxFalloff) 1.0 0.0 1.0 0.0 (Transformation|GetWorldTransform (Variables|Default|GetBox)) "Field_FallOff_None") (Field|SetUniformInteger (Variables|Default|GetUniformInteger) 4) "Field_Culling_Inside")))

(event EventTick
  (params (DeltaSeconds :type Float%20%28single-precision%29)))

(fn ConstructionScript
  (Class|FieldSystemComponent|AddFieldCommand (Variables|Field|GetFieldSystemComponent) true "Field_DynamicState" 0 (Field|SetCullingField (Variables|Default|GetCullingField) (Field|SetBoxFalloff (Variables|Default|GetBoxFalloff) 1.0 0.0 1.0 0.0 (Transformation|GetWorldTransform (Variables|Default|GetBox)) "Field_FallOff_None") (Field|SetUniformInteger (Variables|Default|GetUniformInteger) 4) "Field_Culling_Inside")))