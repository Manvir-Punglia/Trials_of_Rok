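; Tutorial event manager that drives Muninn, the hover-text bird guide, and tracks tutorial completion.
; Tutorial objects call collision, hit or lock-on events, which store a position and dialogue index, then blank and deactivate Muninn.
; The bird's AnimNotify triggers MuninnSpeak to apply both and reactivate it.
; Lock-on marks completion, saved to TutorialFin only when creating a new save; BeginPlay teleports players who completed it to Playerspawn.
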(event Custom|DefaultMuninnSpeech
  (bind _muninn (Variables|Default|GetMuninn))
  ;[1 1 1] sets bird text to blank then sets bird to inactive which will trigger below
  (Default|SetBlank _muninn)
  (Default|SetActive _muninn false))

(event Custom|MuninnSpeak
  (bind _muninn (Variables|Default|GetMuninn))
  ;[1 1 1] triggered via AnimNotify in bird, updats position, dialogue, and sets it back to active
  (Default|NextPosition _muninn (Variables|Default|GetBirdPos))
  (Default|NextDialog _muninn (Variables|Default|GetdialogueNum))
  (Default|SetActive _muninn true))

(event Custom|setHasCompleted
  (params (completed :type Boolean))
  (bind _returnvalue (SaveGame|DoesSaveGameExist "TutorialFin"))
  (if _returnvalue
    (bind _returnvalue_2 (SaveGame|LoadGamefromSlot "TutorialFin"))
    (bind _asbp_save (Utilities|Casting|CastToBP_Save _returnvalue_2))
    (bind _output_get (Variables|/Game/Dynamic/Blueprints/BP_Save.BP_Save_C|SethasComplete _asbp_save completed))
    (Development|PrintString (Utilities|String|Append "Setting tutorial completion to: " (Utilities|String|ToString(Boolean) _output_get)))
    (else
      (bind _returnvalue_3 (SaveGame|CreateSaveGameObject "/Game/Dynamic/Blueprints/BP_Save.BP_Save_C"))
      (Variables|/Game/Dynamic/Blueprints/BP_Save.BP_Save_C|SethasComplete _returnvalue_3 completed)
      (bind _returnvalue_4 (SaveGame|SaveGametoSlot _returnvalue_3 "TutorialFin"))
      (Development|PrintString (Utilities|String|Append "Setting tutorial completion to: " (Utilities|String|ToString(Boolean) _returnvalue_4))))))

(event EventBeginPlay
  ;[1 1 1] Creates a reference to the tutorial npc on begin
  (bind _returnvalue (Actor|GetActorOfClass "/Game/Dynamic/Blueprints/NPC_BP/BP_HoverTextActor.BP_HoverTextActor_C"))
  (Variables|Default|SetMuninn _returnvalue)
  (bind _returnvalue_2 (SaveGame|LoadGamefromSlot "TutorialFin"))
  (Utilities|IsValid _returnvalue_2
    (:Is%20Valid
      (bind _asbp_save (Utilities|Casting|CastToBP_Save _returnvalue_2))
      (if (Variables|/Game/Dynamic/Blueprints/BP_Save.BP_Save_C|GethasComplete _asbp_save)
        (Development|PrintString (Utilities|String|ToString(Boolean) (Variables|/Game/Dynamic/Blueprints/BP_Save.BP_Save_C|GethasComplete _asbp_save)))
        (Transformation|SetWorldLocation (Variables|/Script/Engine.Actor|GetRootComponent (Game|GetPlayerCharacter 0)) (Variables|Default|Getplayerspawn) false false)))))

(event EventCollisionEvent
  (params (NewPos :type Vector :default "0, 0, 0") (NewDialogueNum :type Integer))
  ;[1 1 1] when the events get called by the tutorial objects, update the bird position and dialogue num then call retrospective events (different event types are seperated in case we want different things to happen from the different events)
  (Variables|Default|SetBirdPos NewPos)
  (Variables|Default|SetdialogueNum NewDialogueNum)
  (CallFunction|DefaultMuninnSpeech))

(event EventHitEvent
  (params (NewPos :type Vector :default "0, 0, 0") (NewDialogueNum :type Integer))
  ;[1 1 1] when the events get called by the tutorial objects, update the bird position and dialogue num then call retrospective events (different event types are seperated in case we want different things to happen from the different events)
  (Variables|Default|SetBirdPos NewPos)
  (Variables|Default|SetdialogueNum NewDialogueNum)
  (CallFunction|DefaultMuninnSpeech))

(event EventLockonEvent
  (params (NewPos :type Vector :default "0, 0, 0") (NewDialogueNum :type Integer))
  ;[1 1 1] when the events get called by the tutorial objects, update the bird position and dialogue num then call retrospective events (different event types are seperated in case we want different things to happen from the different events)
  (Variables|Default|SetBirdPos NewPos)
  (Variables|Default|SetdialogueNum NewDialogueNum)
  (CallFunction|SetHasCompleted true)
  (CallFunction|DefaultMuninnSpeech))

(fn ConstructionScript)