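; Tutorial object that fires a one-time event when the player locks on to it.
; When the player's lock-on call arrives, it shows or hides its lock-on widget to match the lock state.
; The first lock-on sends its bird position and dialogue number to the BP_TutorialEventManager found at BeginPlay, then sets a flag so it never repeats.
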(event EventBeginPlay
  ;[1 1 1] on begin, create reference to the tutorial event manager
  (bind _returnvalue (Actor|GetActorOfClass "/Game/Dynamic/Blueprints/TutorialObjects/BP_TutorialEventManager.BP_TutorialEventManager_C"))
  (Variables|Default|SetTutorialEventManagerRef _returnvalue))

(event EventLockedon
  (params (LockedOn? :type Boolean))
  (bind _lockonwidget (Variables|Default|GetLockOnWidget))
  ;[1 1 1] when the locked on event gets called via the player, check to see if lock on event has been triggered already and if it hasn't, send position and dialogue updates through to the tutorial event manager via the event interface then set internal event trigger variable to true
  (if LockedOn?
    (Development|SetHiddeninGame _lockonwidget false false)
    (if (not (Variables|Default|GethasTriggeredEvent))
      (Default|LockonEvent (Variables|Default|GetTutorialEventManagerRef) (Variables|Default|GetBirdPos) (Variables|Default|GetDialogueNum))
      (Variables|Default|SethasTriggeredEvent true))
    (else
      (Development|SetHiddeninGame _lockonwidget true false))))

(fn ConstructionScript)